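; Player controller that shows the mouse cursor at start and handles cursor and menu toggling through Enhanced Input actions.
; IA_Show_Mous flips cursor visibility along with the input mode, switching between Game Only and Game and UI.
; IA_Menu opens WB_Menu with a Tower reference, turning the cursor on if its flag is off.
; Closing the menu removes all widgets and leaves the cursor state unchanged, with no game pause involved.
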(event Custom|E_Show_Mous
  (bind _self self)
  (if (Variables|Default|GetB_Show_Mous)
    (Variables|Default|SetbShowMouseCursor false)
    (Variables|Default|SetB_Show_Mous false)
    (Input|SetInputModeGameOnly _self false)
    (else
      (Variables|Default|SetbShowMouseCursor true)
      (Variables|Default|SetB_Show_Mous true)
      (Input|SetInputModeGameandUI _self 0 "DoNotLock" true false))))

(event Input|EnhancedActionEvents|EnhancedInputActionIA_Show_Mous
  (params (ActionValue :type Boolean) (ElapsedSeconds :type Float%20%28double-precision%29) (TriggeredSeconds :type Float%20%28double-precision%29) (InputAction :type Input%20Action%20Object%20Reference :default "/Game/Input/IA_Show_Mous.IA_Show_Mous"))
  (:Started
    (CallFunction|EShowMous)))

(event Input|EnhancedActionEvents|EnhancedInputActionIA_Menu
  (params (ActionValue :type Boolean) (ElapsedSeconds :type Float%20%28double-precision%29) (TriggeredSeconds :type Float%20%28double-precision%29) (InputAction :type Input%20Action%20Object%20Reference :default "/Game/Input/IA_Menu.IA_Menu"))
  (:Started
    (if (Variables|Default|GetB_Puse_Menu)
      (Variables|Default|SetB_Puse_Menu false)
      (Viewport|RemoveAllWidgets)
      (else
        (if (Variables|Default|GetB_Show_Mous)
          _
          (else
            (CallFunction|EShowMous)))
        (Variables|Default|SetB_Puse_Menu true)
        (bind _returnvalue (UserInterface|CreateWidget "/Game/Widjet/WB_Menu.WB_Menu_C" 0 (Variables|Default|GetTower)))
        (UserInterface|Viewport|AddtoViewport _returnvalue 0)))))

(event EventBeginPlay
  (Variables|Default|SetbShowMouseCursor true))

(fn ConstructionScript)