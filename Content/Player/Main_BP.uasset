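; Player camera Blueprint that provides mouse-driven look and zoom.
; On BeginPlay it passes its ATower reference to the Main_Player_Controller_BP.
; Look input rotates the Point component with clamped pitch and free yaw, requiring the mouse-press action only while the cursor flag BShowMous is set.
; Scroll input zooms by adjusting the camera's field of view within limits, with both inputs scaled by delta time.
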(event Input|EnhancedActionEvents|EnhancedInputActionIA_Look
  (params (ActionValue :type Vector%202D%20Structure) (ElapsedSeconds :type Float%20%28double-precision%29) (TriggeredSeconds :type Float%20%28double-precision%29) (InputAction :type Input%20Action%20Object%20Reference :default "/Game/Input/IA_Look.IA_Look"))
  (bind _returnvalue (Utilities|Time|GetWorldDeltaSeconds))
  (bind _point (Variables|Default|GetPoint))
  (bind _m_p_c (Variables|Default|GetM_P_C))
  (bind _b_show_mous (Variables|/Script/Tower_Project.Main_Player_Controller|GetB_Show_Mous _m_p_c))
  (bind _relativerotation (Variables|/Script/Engine.SceneComponent|GetRelativeRotation _point))
  (if (or (and (Input|EnhancedActionValues|GetIA_Perss_Mous) _b_show_mous) (not _b_show_mous))
    (Transformation|SetRelativeRotation _point (Math|Rotator|MakeRotator 0.0 (Math|Float|Clamp(Float) (+ (* (.y ActionValue) _returnvalue 4e+01) (.pitch _relativerotation)) -89.0 3e+01) (+ (.yaw _relativerotation) (* (.x ActionValue) _returnvalue 4e+01))) false false)))

(event Input|EnhancedActionEvents|EnhancedInputActionIA-Scroll
  (params (ActionValue :type Float%20%28double-precision%29) (ElapsedSeconds :type Float%20%28double-precision%29) (TriggeredSeconds :type Float%20%28double-precision%29) (InputAction :type Input%20Action%20Object%20Reference :default "/Game/Input/IA-Scroll.IA-Scroll"))
  (bind _camera (Variables|Default|GetCamera))
  (Camera|SetFieldOfView _camera (Math|Float|Clamp(Float) (+ (Variables|/Script/Engine.CameraComponent|GetFieldOfView _camera) (* ActionValue -8e+01 (Utilities|Time|GetWorldDeltaSeconds))) 4e+01 1.2e+02)))

(event EventBeginPlay
  (bind _asmain_player_controller_bp (Utilities|Casting|CastToMain_Player_Controller_BP (Game|GetPlayerController 0)))
  (Variables|/Script/Tower_Project.Main_Player_Controller|SetTower _asmain_player_controller_bp (Variables|Default|GetATower)))

(fn ConstructionScript)